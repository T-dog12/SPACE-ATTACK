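; BP_Tank_Enemy_AimAt is an enemy tank variant that fires projectiles aimed directly at its hunt target.
; Its Attack event checks that HuntTarget is valid, then spawns a BP_FastProjectile at the FireDirection component, rotated to look at the target's current location.
; It then sets the collision object type of the projectile's SMSphere to a custom game channel.
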(event EventBeginPlay
  (|CallParentFunction) ; This node is disabled and will not be called.\nDrag off pins to build functionality.
)

(event Collision|EventActorBeginOverlap
  (params (OtherActor :type Actor%20Object%20Reference)))

(event EventTick
  (params (DeltaSeconds :type Float%20%28single-precision%29))
  (|CallParentFunction DeltaSeconds) ; This node is disabled and will not be called.\nDrag off pins to build functionality.
)

(event EventAttack
  (bind _hunttarget (Variables|Default|GetHuntTarget))
  (bind _firedirection (Variables|Default|GetFireDirection))
  (bind _returnvalue (Transformation|GetWorldLocation _firedirection))
  (Utilities|IsValid _hunttarget
    (:Is%20Valid
      (bind _returnvalue_2 (Game|SpawnActorfromClass "/Game/StudentWork/Blueprints/Projectiles/BP_FastProjectile.BP_FastProjectile_C" (Math|Transform|MakeTransform _returnvalue (Math|Rotator|FindLookatRotation _returnvalue (Transformation|GetActorLocation _hunttarget)) "1.000000,1.000000,1.000000") "Undefined" "MultiplyWithRoot" 0 0))
      (Collision|SetCollisionObjectType (Variables|/Game/StudentWork/Blueprints/Projectiles/BP_FastProjectile.BP_FastProjectile_C|GetSM_Sphere _returnvalue_2) "ECC_GameTraceChannel2"))))

(fn ConstructionScript
  (|CallParentFunction))