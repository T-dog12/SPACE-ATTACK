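; BP_Turret is a destructible enemy turret hazard that tracks and shoots at the player ship.
; A capsule overlap with the ship stores it as the target and starts a looping fire timer, which any end overlap clears without clearing the target.
; Each tick it smoothly rotates toward a fixed offset ahead of the ship's body to lead shots.
; Bullets spawn enlarged on their own collision channel; depleted health triggers a Niagara explosion.
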(event OnComponentBeginOverlap(Capsule)
  (params (OverlappedComponent :type Primitive%20Component%20Object%20Reference) (OtherActor :type Actor%20Object%20Reference) (OtherComp :type Primitive%20Component%20Object%20Reference) (OtherBodyIndex :type Integer) (bFromSweep :type Boolean) (SweepResult :type Hit%20Result%20Structure%20%28by%20ref%29))
  (bind _asbp_player_ship (Utilities|Casting|CastToBP_PlayerShip OtherActor))
  (Variables|Default|SetDetectedObject _asbp_player_ship)
  (bind _returnvalue (Utilities|Time|SetTimerbyEvent (delegate Custom|Fire) 0.25 true))
  (Variables|Default|SetFireCooldown _returnvalue))

(event OnComponentEndOverlap(Capsule)
  (params (OverlappedComponent :type Primitive%20Component%20Object%20Reference) (OtherActor :type Actor%20Object%20Reference) (OtherComp :type Primitive%20Component%20Object%20Reference) (OtherBodyIndex :type Integer))
  (Utilities|Time|ClearandInvalidateTimerbyHandle (Variables|Default|GetFireCooldown)))

(event Custom|RotateTo
  (bind _newparam (CallFunction|GetPointto))
  (Transformation|SetWorldRotation (Variables|Default|GetRotator) (Math|Interpolation|RInterpTo (Transformation|GetWorldRotation (Variables|Default|GetRotator)) _newparam (Utilities|Time|GetWorldDeltaSeconds) 1e+01) false false))

(event Custom|Fire
  (bind _firepoint (Variables|Default|GetFirePoint))
  (bind _returnvalue (Game|SpawnActorfromClass "/Game/StudentWork/Blueprints/Projectiles/BP_ShipBullet.BP_ShipBullet_C" (Math|Transform|MakeTransform (Transformation|GetWorldLocation _firepoint) (Transformation|GetWorldRotation _firepoint) "10.000000,10.000000,10.000000") "Undefined" "MultiplyWithRoot" 0 0))
  (Collision|SetCollisionObjectType (Variables|/Game/StudentWork/Blueprints/Projectiles/BP_ShipBullet.BP_ShipBullet_C|GetSphere _returnvalue) "ECC_GameTraceChannel2"))

(event Game|Damage|EventAnyDamage
  (params (Damage :type Float%20%28single-precision%29) (DamageType :type Damage%20Type%20Object%20Reference) (InstigatedBy :type Controller%20Object%20Reference) (DamageCauser :type Actor%20Object%20Reference))
  (bind _output_get (Variables|Default|SetHealth (- (Variables|Default|GetHealth) Damage)))
  (if (<= _output_get 0.0)
    (Niagara|SpawnSystematLocation "/Game/StudentWork/FX/Explosions/NI_ExplosionFire.NI_ExplosionFire" (Transformation|GetWorldLocation (Variables|Default|GetDefaultSceneRoot)))
    (Actor|DestroyActor)))

(event EventTick
  (params (DeltaSeconds :type Float%20%28single-precision%29))
  (Utilities|IsValid (Variables|Default|GetDetectedObject)
    (:Is%20Valid
      (CallFunction|Rotateto))))

(fn ConstructionScript)

(fn GetPointto
  (bind _detectedobject (Variables|Default|GetDetectedObject))
  (bind _body (Variables|/Game/StudentWork/Blueprints/BP_PlayerShip.BP_PlayerShip_C|GetBody _detectedobject))
  (return (Math|Rotator|FindLookatRotation (Transformation|GetWorldLocation (Variables|Default|GetRotator)) (+ (Transformation|GetWorldLocation _body) (* (Math|Vector|GetForwardVector _body) 7.5e+03)))))