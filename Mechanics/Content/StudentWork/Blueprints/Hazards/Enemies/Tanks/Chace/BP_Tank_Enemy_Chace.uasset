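; Chasing tank enemy that hunts the player once they enter its sight sphere.
; Overlap stores the player as target, widens the sphere from MinSight to MaxSight and starts movement and attack timers.
; Move uses AI MoveTo toward the target while it overlaps, otherwise shrinks the sphere and pauses both timers.
; Despite its name, OutOfSight returns true while the target is inside the sphere.
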(event OnComponentBeginOverlap(Sphere)
  (params (OverlappedComponent :type Primitive%20Component%20Object%20Reference) (OtherActor :type Actor%20Object%20Reference) (OtherComp :type Primitive%20Component%20Object%20Reference) (OtherBodyIndex :type Integer) (bFromSweep :type Boolean) (SweepResult :type Hit%20Result%20Structure%20%28by%20ref%29))
  (bind _asbp_player_character (Utilities|Casting|CastToBP_PlayerCharacter OtherActor))
  (Variables|Default|SetHuntTarget _asbp_player_character)
  (Components|Sphere|SetSphereRadius (Variables|Default|GetSphere) (Variables|Default|GetMaxSight) true)
  (CallFunction|StartMovementTimer)
  (CallFunction|StartAttackTimer))

(event EventMove
  (bind _hunttarget (Variables|Default|GetHuntTarget))
  (bind _isoverlapped (CallFunction|OutOfSight))
  (if _isoverlapped
    (Utilities|IsValid _hunttarget
      (:Is%20Valid
        (AI|AIMoveTo self (Transformation|GetWorldLocation (Variables|/Game/Blueprints/BP_PlayerCharacter.BP_PlayerCharacter_C|GetBodyMesh _hunttarget)) 0 3e+02 false)))
    (else
      (Components|Sphere|SetSphereRadius (Variables|Default|GetSphere) (Variables|Default|GetMinSight) true)
      (Utilities|Time|PauseTimerbyHandle (Variables|Default|GetAttack%20Timer))
      (Utilities|Time|PauseTimerbyHandle (Variables|Default|GetMovementTimer)))))

(fn ConstructionScript
  (Transformation|SetWorldRotation (Variables|Default|GetTankMesh) (Transformation|GetWorldRotation (Variables|Default|GetCapsuleComponent)) false false)
  (|CallParentFunction))

(fn OutOfSight
  (return (Collision|IsOverlappingActor (Variables|Default|GetSphere) (Variables|Default|GetHuntTarget) :!class /Script/Engine.PrimitiveComponent)))