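; Tank enemy variant that fires fast projectiles in random horizontal directions.
; Its Attack event spawns a BP_FastProjectile at the FireDirection component's location, using only the yaw from a random rotator so pitch and roll stay flat.
; It then switches the projectile's sphere mesh to a custom collision object channel.
; The event graph holds no other active logic, and the construction script only calls the parent.
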(event EventBeginPlay
  (|CallParentFunction) ; This node is disabled and will not be called.\nDrag off pins to build functionality.
)

(event Collision|EventActorBeginOverlap
  (params (OtherActor :type Actor%20Object%20Reference)))

(event EventTick
  (params (DeltaSeconds :type Float%20%28single-precision%29))
  (|CallParentFunction DeltaSeconds) ; This node is disabled and will not be called.\nDrag off pins to build functionality.
)

(event EventAttack
  (bind _returnvalue (Game|SpawnActorfromClass "/Game/StudentWork/Blueprints/Projectiles/BP_FastProjectile.BP_FastProjectile_C" (Math|Transform|MakeTransform (Transformation|GetWorldLocation (Variables|Default|GetFireDirection)) (Math|Rotator|MakeRotator 0.0 0.0 (.yaw (Math|Random|RandomRotator true))) "1.000000,1.000000,1.000000") "Undefined" "MultiplyWithRoot" 0 0))
  (Collision|SetCollisionObjectType (Variables|/Game/StudentWork/Blueprints/Projectiles/BP_FastProjectile.BP_FastProjectile_C|GetSM_Sphere _returnvalue) "ECC_GameTraceChannel2"))

(fn ConstructionScript
  (|CallParentFunction))