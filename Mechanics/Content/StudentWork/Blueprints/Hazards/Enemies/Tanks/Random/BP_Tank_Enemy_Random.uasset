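; BP_Tank_Enemy_Random is a tank enemy hazard that roams to a random point and attacks the player on proximity.
; On BeginPlay, its Move event sends it by AI MoveTo to a random navigable location within a fixed radius, with no repeat wired in this graph.
; When BP_PlayerCharacter overlaps its Sphere, it stores the player as HuntTarget and starts the attack timer.
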(event OnComponentBeginOverlap(Sphere)
  (params (OverlappedComponent :type Primitive%20Component%20Object%20Reference) (OtherActor :type Actor%20Object%20Reference) (OtherComp :type Primitive%20Component%20Object%20Reference) (OtherBodyIndex :type Integer) (bFromSweep :type Boolean) (SweepResult :type Hit%20Result%20Structure%20%28by%20ref%29))
  (bind _asbp_player_character (Utilities|Casting|CastToBP_PlayerCharacter OtherActor))
  (Variables|Default|SetHuntTarget _asbp_player_character)
  (CallFunction|StartAttackTimer))

(event EventBeginPlay
  (CallFunction|Move))

(event EventMove
  (bind _randomlocation (Class|NavigationSystemV1|GetRandomLocationinNavigableRadius (Transformation|GetActorLocation) 5e+02 0 0))
  (AI|AIMoveTo self _randomlocation 0 5.0 false))

(fn ConstructionScript
  (|CallParentFunction))