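; BP_Debris is a hazard actor that damages the player ship on collision and can itself be destroyed by damage.
; Hits on a BP_PlayerShip apply fixed damage, then share a path with any received damage that spawns a Niagara rock explosion and destroys the debris.
; The construction script picks a random mesh from PossibleMeshes and gives it a random rotation for visual variety.
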(event OnComponentHit(StaticMesh)
  (params (HitComponent :type Primitive%20Component%20Object%20Reference) (OtherActor :type Actor%20Object%20Reference) (OtherComp :type Primitive%20Component%20Object%20Reference) (NormalImpulse :type Vector :default "0, 0, 0") (Hit :type Hit%20Result%20Structure%20%28by%20ref%29))
  (bind _asbp_player_ship (Utilities|Casting|CastToBP_PlayerShip OtherActor))
  (Game|Damage|ApplyDamage _asbp_player_ship 1e+01 0 0)
  (Niagara|SpawnSystematLocation "/Game/StudentWork/FX/Explosions/NI_RockExplosion.NI_RockExplosion" (Transformation|GetWorldLocation (Variables|Default|GetStaticMesh)))
  (Actor|DestroyActor))

(event Game|Damage|EventAnyDamage
  (params (Damage :type Float%20%28single-precision%29) (DamageType :type Damage%20Type%20Object%20Reference) (InstigatedBy :type Controller%20Object%20Reference) (DamageCauser :type Actor%20Object%20Reference))
  (Niagara|SpawnSystematLocation "/Game/StudentWork/FX/Explosions/NI_RockExplosion.NI_RockExplosion" (Transformation|GetWorldLocation (Variables|Default|GetStaticMesh)))
  (Actor|DestroyActor))

(fn ConstructionScript
  (bind _possiblemeshes (Variables|Default|GetPossibleMeshes))
  (bind _staticmesh (Variables|Default|GetStaticMesh))
  (Components|StaticMesh|SetStaticMesh _staticmesh (Utilities|Array|Get(acopy) _possiblemeshes (Math|Random|RandomInteger (Utilities|Array|Length _possiblemeshes))))
  (Transformation|SetWorldRotation _staticmesh (Math|Random|RandomRotator false) false false))