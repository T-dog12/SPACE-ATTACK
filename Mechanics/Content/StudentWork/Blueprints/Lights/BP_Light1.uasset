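; BP_Light1 is a light Blueprint that pulses the intensity of its point light while Active is set.
; Each Tick, a Reverse flag selects whether the LIGHT timeline plays forward (when true) or backward.
; The timeline track drives a Lerp between a dim and a bright intensity, and its Finished output flips the flag to swap direction.
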(event EventTick
  (params (DeltaSeconds :type Float%20%28single-precision%29))
  (if (Variables|Default|GetActive)
    (if (Variables|Default|GetReverse)
      (bind _newtrack_0 (Timeline|LIGHT Play)
        (:Update
          (Rendering|Components|Light|SetIntensity (Variables|Default|GetPointLight) (Math|Float|Lerp 3e+02 7.5e+02 _newtrack_0)))
        (:Finished
          (Variables|Default|SetReverse (not (Variables|Default|GetReverse)))))
      (else
        (Timeline|LIGHT Reverse)))))

(fn ConstructionScript)