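; Player-controlled ship that flies constantly forward, with Enhanced Input for pitch, roll and firing.
; Tick overrides the physics body's velocity along its forward vector, while pitch and roll apply acceleration-based torque scaled by input.
; Firing runs a debug-drawn line trace from the Arrow component and applies damage to the hit actor.
; Taking damage triggers a camera shake.
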(event Input|EnhancedActionEvents|EnhancedInputActionIA_Pitch
  (params (ActionValue :type Float%20%28double-precision%29) (ElapsedSeconds :type Float%20%28double-precision%29) (TriggeredSeconds :type Float%20%28double-precision%29) (InputAction :type Input%20Action%20Object%20Reference :default "/Game/StudentWork/Input/IA_Pitch.IA_Pitch"))
  (bind _body (Variables|Default|GetBody))
  ;[0.15 0.15 0.15 0.5] Movement
  (Class|PrimitiveComponent|AddTorqueinDegrees _body (* (Math|Vector|GetRightVector _body) (Math|Float|Lerp 0.0 (Variables|Default|GetMaxTorque) ActionValue)) "None" true))

(event Input|EnhancedActionEvents|EnhancedInputActionIA_Roll
  (params (ActionValue :type Float%20%28double-precision%29) (ElapsedSeconds :type Float%20%28double-precision%29) (TriggeredSeconds :type Float%20%28double-precision%29) (InputAction :type Input%20Action%20Object%20Reference :default "/Game/StudentWork/Input/IA_Roll.IA_Roll"))
  (bind _body (Variables|Default|GetBody))
  ;[0.15 0.15 0.15 0.5] Movement
  (Class|PrimitiveComponent|AddTorqueinDegrees _body (* (Math|Vector|GetForwardVector _body) (Math|Float|Lerp 0.0 (Variables|Default|GetMaxTorque) ActionValue)) "None" true))

(event Input|EnhancedActionEvents|EnhancedInputActionIA_Fire
  (params (ActionValue :type Boolean) (ElapsedSeconds :type Float%20%28double-precision%29) (TriggeredSeconds :type Float%20%28double-precision%29) (InputAction :type Input%20Action%20Object%20Reference :default "/Game/StudentWork/Input/IA_Fire.IA_Fire"))
  (bind _arrow (Variables|Default|GetArrow))
  (bind _returnvalue (Transformation|GetWorldLocation _arrow))
  (bind _outhit (Collision|LineTraceByChannel _returnvalue (+ _returnvalue (* (Math|Vector|GetForwardVector _arrow) 1e+04)) "TraceTypeQuery1" false 0 "ForDuration"))
  (Game|Damage|ApplyDamage (.HitActor (Collision|BreakHitResult _outhit)) 1e+01 0 0))

(event EventBeginPlay
  ;[0.15 0.15 0.15 0.5] Input Setup
  (bind _asbp_mech_player_controller (Utilities|Casting|CastToBP_MechPlayerController (Game|GetPlayerController 0)))
  (Input|AddMappingContext (PlayerController|LocalPlayerSubsystems|GetEnhancedInputLocalPlayerSubsystem _asbp_mech_player_controller) "/Game/StudentWork/Input/IMC_Ship.IMC_Ship" 0 "(bIgnoreAllPressedKeysUntilRelease=True,bForceImmediately=False,bNotifyUserSettings=False)"))

(event EventTick
  (params (DeltaSeconds :type Float%20%28single-precision%29))
  (bind _body (Variables|Default|GetBody))
  ;[0.15 0.15 0.15 0.5] Movement
  (Physics|SetPhysicsLinearVelocity _body (* (Math|Vector|GetForwardVector _body) 1e+03) false "None"))

(event Game|Damage|EventAnyDamage
  (params (Damage :type Float%20%28single-precision%29) (DamageType :type Damage%20Type%20Object%20Reference) (InstigatedBy :type Controller%20Object%20Reference) (DamageCauser :type Actor%20Object%20Reference))
  (CameraShakes|StartCameraShake (Game|GetPlayerCameraManager 0) "/Game/StudentWork/Blueprints/CamShake/BP_DamageShake.BP_DamageShake_C" 1.0 "CameraLocal" "0, 0, 0"))

(fn ConstructionScript)