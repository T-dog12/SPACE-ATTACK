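; Asteroid cluster placement helper that scatters the Box's child components as spawn points for BP_Debris, then destroys itself on BeginPlay.
; The construction script runs Scatter, randomizing each child's location within Radius of the Box; RandomSize picks a new Radius and scatters again.
; SpawnDebris spawns debris at each child's transform, with random scale chained across axes to keep proportions similar.
; Nothing here calls SpawnDebris or RandomSize, and the box-extent update is disconnected.
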(event Custom|Spawn%20Debris
  (bind _returnvalue (Math|Random|RandomFloatinRange 0.5 7.5))
  (bind _returnvalue_2 (- _returnvalue 1.0))
  (bind _returnvalue_3 (+ _returnvalue 1.0))
  (bind _returnvalue_4 (Math|Random|RandomFloatinRange _returnvalue_2 _returnvalue_3))
  (for _array_element (Components|GetChildrenComponents (Variables|Default|GetBox) false)
    (bind _returnvalue_5 (Game|SpawnActorfromClass "/Game/StudentWork/Blueprints/Hazards/BP_Debris.BP_Debris_C" (Transformation|GetWorldTransform _array_element) "Undefined" "MultiplyWithRoot" 0 0))
    (Transformation|SetWorldScale3D (Variables|/Script/Engine.Actor|GetRootComponent _returnvalue_5) (Math|Vector|MakeVector _returnvalue _returnvalue_4 (Math|Random|RandomFloatinRange (- _returnvalue_4 1.0) (+ _returnvalue_4 1.0))))))

(event Custom|Random%20Size
  (Variables|Default|SetRadius (Math|Random|RandomFloatinRange 2e+03 1e+04))
  (CallFunction|Scatter))

(event EventBeginPlay
  (Actor|DestroyActor))

(fn ConstructionScript
  (CallFunction|Scatter))

(fn Scatter
  (bind _radius (Variables|Default|GetRadius))
  (bind _returnvalue (* _radius -1.0))
  (for _array_element (Components|GetChildrenComponents (Variables|Default|GetBox) false)
    (Transformation|SetWorldLocation _array_element (+ (Transformation|GetWorldLocation (Variables|Default|GetBox)) (Math|Vector|MakeVector (Math|Random|RandomFloatinRange _returnvalue _radius) (Math|Random|RandomFloatinRange _returnvalue _radius) (Math|Random|RandomFloatinRange _returnvalue _radius))) false false)))