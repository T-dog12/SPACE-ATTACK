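; BP_Target is a destructible target that flashes and explodes the first time it takes damage.
; The construction script creates a dynamic flash material instance on the second material slot of its static mesh.
; A DoOnce gate on AnyDamage plays a timeline that drives that material's FlashLevel parameter.
; When the timeline finishes, a Niagara fire explosion spawns at the mesh's location and the actor destroys itself.
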(event Game|Damage|EventAnyDamage
  (params (Damage :type Float%20%28single-precision%29) (DamageType :type Damage%20Type%20Object%20Reference) (InstigatedBy :type Controller%20Object%20Reference) (DamageCauser :type Actor%20Object%20Reference))
  (Utilities|FlowControl|DoOnce false
    (:Completed
      (bind _newtrack_0 (Timeline|Flash PlayFromStart)
        (:Update
          (Rendering|Material|SetScalarParameterValue (Variables|Default|GetFlash%20Material) "FlashLevel" _newtrack_0 :!class /Script/Engine.MaterialInstanceDynamic))
        (:Finished
          (Niagara|SpawnSystematLocation "/Game/StudentWork/FX/Explosions/NI_ExplosionFire.NI_ExplosionFire" (Transformation|GetWorldLocation (Variables|Default|GetStaticMesh)))
          (Actor|DestroyActor))))))

(fn ConstructionScript
  (bind _returnvalue (Rendering|Material|CreateDynamicMaterialInstance (Variables|Default|GetStaticMesh) 1 "/Game/StudentWork/Materials/M_BarralFlash.M_BarralFlash" "None" :!class /Script/Engine.PrimitiveComponent))
  (Variables|Default|SetFlash%20Material _returnvalue))