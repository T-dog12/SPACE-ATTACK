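; Basic enemy tank that chases and shoots at the player once detected.
; A player entering the sight sphere becomes HuntTarget, widens the sphere to MaxSight and starts the movement and attack timers.
; Move pursues the target while it overlaps the sphere, otherwise shrinks it to MinSight; OutOfSight returns true while overlapping, despite its name.
; Attack spawns a fast projectile at FireArrow and sets its collision channel, without checking sight.
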(event OnComponentBeginOverlap(Sphere)
  (params (OverlappedComponent :type Primitive%20Component%20Object%20Reference) (OtherActor :type Actor%20Object%20Reference) (OtherComp :type Primitive%20Component%20Object%20Reference) (OtherBodyIndex :type Integer) (bFromSweep :type Boolean) (SweepResult :type Hit%20Result%20Structure%20%28by%20ref%29))
  (bind _asbp_player_character (Utilities|Casting|CastToBP_PlayerCharacter OtherActor))
  (Variables|Default|SetHuntTarget _asbp_player_character)
  (Components|Sphere|SetSphereRadius (Variables|Default|GetSphere) (Variables|Default|GetMaxSight) true)
  (CallFunction|StartMovementTimer)
  (CallFunction|StartAttackTimer))

(event EventMove
  (bind _hunttarget (Variables|Default|GetHuntTarget))
  (bind _isoverlapped (CallFunction|OutOfSight))
  (if _isoverlapped
    (Utilities|IsValid _hunttarget
      (:Is%20Valid
        (AI|AIMoveTo self "0.000000,0.000000,0.000000" _hunttarget 5.0 false)))
    (else
      (Components|Sphere|SetSphereRadius (Variables|Default|GetSphere) (Variables|Default|GetMinSight) true))))

(event EventAttack
  (bind _firearrow (Variables|Default|GetFireArrow))
  (bind _returnvalue (Game|SpawnActorfromClass "/Game/StudentWork/Blueprints/Projectiles/BP_FastProjectile.BP_FastProjectile_C" (Math|Transform|MakeTransform (Transformation|GetWorldLocation _firearrow) (Transformation|GetWorldRotation _firearrow) "1.000000,1.000000,1.000000") "Undefined" "MultiplyWithRoot" 0 0))
  (Collision|SetCollisionObjectType (Variables|/Game/StudentWork/Blueprints/Projectiles/BP_FastProjectile.BP_FastProjectile_C|GetSM_Sphere _returnvalue) "ECC_GameTraceChannel2"))

(fn ConstructionScript
  (|CallParentFunction))

(fn OutOfSight
  (return (Collision|IsOverlappingActor (Variables|Default|GetSphere) (Variables|Default|GetHuntTarget) :!class /Script/Engine.PrimitiveComponent)))