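; MechGameMode is a game mode Blueprint that tracks the remaining enemy bases and triggers the player's win condition.
; On BeginPlay it caches player 0's pawn as a BP_PlayerShip and counts all BP_EnemyBase actors in the level.
; Each BaseDistroyed event decrements that count and calls WinScreen on the player ship once none remain.
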(event Custom|BaseDistroyed
  (bind _output_get (Variables|Default|SetNumBases (- (Variables|Default|GetNumBases) 1)))
  (if (<= _output_get 0)
    (Default|WinScreen (Variables|Default|GetPlayerShip))))

(event EventBeginPlay
  (bind _asbp_player_ship (Utilities|Casting|CastToBP_PlayerShip (Game|Player|GetPlayerPawn 0))
    (:then
      (Variables|Default|SetPlayerShip _asbp_player_ship))
    (:CastFailed
      _))
  (bind _outactors (Actor|GetAllActorsOfClass "/Game/StudentWork/Blueprints/Houses/BP_EnemyBase.BP_EnemyBase_C"))
  (Variables|Default|SetNumBases (Utilities|Array|Length _outactors)))

(fn ConstructionScript)